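; Health component that tracks an actor's current health and signals when it dies.
; Current health starts at the maximum on BeginPlay, and the Damage and Heal functions adjust it, clamped between zero and the maximum.
; Damage calls the OnDeath dispatcher whenever health is at zero afterward, with no guard against repeat calls on further hits.
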(event `self.ReceiveBeginPlay`
  (set `self.ActualHealth` (`self.MaxHealth`)))

(fn `damage`
  (params (damageAmount :type "Float (double-precision)"))
  (bind _output_get (set `self.ActualHealth` (`KismetMathLibrary.FClamp` (- (`self.ActualHealth`) damageAmount) 0.0 (`self.MaxHealth`))))
  (if (<= _output_get 0.0)
    (`self.OnDeath`)))

(fn `heal`
  (params (healAmount :type "Float (double-precision)"))
  (set `self.ActualHealth` (`KismetMathLibrary.FClamp` (+ (`self.ActualHealth`) healAmount) 0.0 (`self.MaxHealth`))))