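; BP_Enemy is an enemy character that chases the player and damages it on contact.
; A looping timer repeatedly issues an AI MoveTo toward the player character, with Tick left unused.
; Overlapping a BP_TopDownCharacter applies EnemyDamage through that character's health component.
; When its own health component reports death, it calls OnEnemyDeath and destroys itself.
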(event `Follow Player`
  (`|AIMoveTo` self (0.0 0.0 0.0) (`GameplayStatics.GetPlayerCharacter` 0)))

(event `self.ReceiveBeginPlay`
  (`KismetSystemLibrary.K2_SetTimerDelegate` (delegate `Follow Player`) 0.2 true))

(event `self.ReceiveActorBeginOverlap`
  (params (OtherActor :type "Actor Object Reference"))
  (bind _asbp_top_down_character (cast `/Game/TopDown/Blueprints/BP_TopDownCharacter` OtherActor))
  (`self.DamagePlayer` _asbp_top_down_character))

(event `self.BPC_HealthComponent.OnDeath`
  (`self.OnEnemyDeath`)
  (`self.K2_DestroyActor`))

(fn `DamagePlayer`
  (params (Player :type "/Game/TopDown/Blueprints/BP_TopDownCharacter Object Reference"))
  (`/Game/Systems/BPC_HealthComponent.damage` (`/Game/TopDown/Blueprints/BP_TopDownCharacter.BPC_HealthComponent` Player) (`self.Enemy Damage`)))

(fn `UserConstructionScript`)